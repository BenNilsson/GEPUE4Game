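; BP_Player is a player Blueprint that sets up and opens the inventory UI.
; On BeginPlay it creates the inventory widget for player controller 0, adds it to the viewport hidden and initializes it with its InventoryComponent.
; The Inventory input action only toggles the stored widget on, so closing is not handled in this graph.
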(event `InputAction|Inventory`
  (params (Key :type "Key Structure"))
  ;[1 1 1] Open Inventory UI
  (:`Pressed`
    (`/Game/UI/Inventory/Widget_Inventory.ToggleInventory_Event` (`self.InventoryWidget`) true)))

(event `self.ReceiveBeginPlay`
  ;[1 1 1] Add Inventory Widget To Scene
  (bind _returnvalue (`|CreateWidget` "/Game/UI/Inventory/Widget_Inventory.Widget_Inventory_C" (`GameplayStatics.GetPlayerController` 0)))
  (`UserWidget.AddToViewport` _returnvalue 0)
  (bind _output_get (set `self.InventoryWidget` _returnvalue))
  (`/Game/UI/Inventory/Widget_Inventory.ToggleInventory_Event` _output_get false)
  (`/Game/UI/Inventory/Widget_Inventory.InitializeInvUI_Event` (`self.InventoryWidget`) (`self.InventoryComponent`)))

(fn `UserConstructionScript`)