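; Bow weapon Blueprint that computes an arrow aim from the player camera and spawns arrow projectiles.
; HandleCrosshairPosition lowers simulated gravity each call, scaled by a line-trace result, then predicts and debug-draws the projectile path.
; The predicted endpoint orients the spawn transform, so SpawnArrow fires a zero-gravity arrow toward it.
; Fire and release events are bound but empty; the looping aim timer and spawn logic are disconnected.
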(event `OnWeaponFireEvent`)

(event `self.ReceiveBeginPlay`
  (add `WeaponBase.OnWeaponFiredReleasedEvent` (delegate `OnWeaponFireReleasedEvent`))
  (add `WeaponBase.OnWeaponFiredEvent` (delegate `OnWeaponFireEvent`)))

(event `OnWeaponFireReleasedEvent`)

(fn `HandleCrosshairPosition`
  (bind _returnvalue (`SceneComponent.K2_GetComponentLocation` (`self.ArrowComponent`)))
  (bind _transformcomponent (`PlayerCameraManager.TransformComponent` (`PlayerController.PlayerCameraManager` (`GameplayStatics.GetPlayerController` 0))))
  (bind _transformcomponent_2 (`PlayerCameraManager.TransformComponent` (`PlayerController.PlayerCameraManager` (`GameplayStatics.GetPlayerController` 0))))
  (bind _returnvalue_2 (`SceneComponent.K2_GetComponentLocation` _transformcomponent))
  (bind (_outhit _returnvalue_3) (`KismetSystemLibrary.LineTraceSingle` :`Start` _returnvalue_2 :`End` (+ _returnvalue_2 (* (`SceneComponent.GetForwardVector` _transformcomponent) 15000.0)) :`TraceChannel` "TraceTypeQuery3" :`bTraceComplex` true :`DrawTime` 0.1))
  (set `self.GravityIncrement_0` (* (/ 1.0 (`KismetMathLibrary.VSize` (`KismetMathLibrary.SelectVector` (`.ImpactPoint` (`GameplayStatics.BreakHitResult` _outhit)) (/ (* (`SceneComponent.GetForwardVector` (`PlayerCameraManager.TransformComponent` (`PlayerController.PlayerCameraManager` (`GameplayStatics.GetPlayerController` 0)))) 15000.0) (`self.GravitySpeedFactor_0`)) _returnvalue_3))) (`self.GravitySpeedFactor_0`)))
  (set `self.CurrentGravity_0` (`KismetMathLibrary.FClamp` (- (`self.CurrentGravity_0`) (`self.GravityIncrement_0`)) 0.0 (`self.StartGravity_0`)))
  (bind (_outhit_2 _outpathpositions _outlasttracedestination _returnvalue_4) (`GameplayStatics.Blueprint_PredictProjectilePath_ByTraceChannel` :`StartPos` (`SceneComponent.K2_GetComponentLocation` _transformcomponent_2) :`LaunchVelocity` (* (- (`SceneComponent.GetForwardVector` _transformcomponent_2) (`KismetMathLibrary.MakeVector` 0.0 0.0 (`self.CurrentGravity_0`))) 15000.0) :`TraceChannel` "ECC_GameTraceChannel2" :`bTraceComplex` true :`DrawDebugType` "ForOneFrame" :`DrawDebugTime` 1.0 :`SimFrequency` 30.0 :`OverrideGravityZ` (`self.CurrentGravity_0`)))
  (set `self.SpawnLocation_0` (`KismetMathLibrary.MakeTransform` _returnvalue (`KismetMathLibrary.FindLookAtRotation` _returnvalue (`KismetMathLibrary.SelectVector` (`.ImpactPoint` (`GameplayStatics.BreakHitResult` _outhit_2)) _outlasttracedestination _returnvalue_4)))))

(fn `SpawnArrow`
  (params (SpawnLocation :type "Transform Structure"))
  (bind _returnvalue (`|SpawnActorFromClass` (`self.ArrowProjectile`) SpawnLocation "Undefined" "OverrideRootScale" null null))
  (`ArrowProjectile.SetGravity` _returnvalue 0.0))

(fn `UserConstructionScript`)