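; BP_DeerAIController is the deer's AI controller, translating perception updates into Blackboard values.
; Each update branches on sense class: sight writes the stimulus actor to PlayerActor, while hearing writes the stimulus location to NoiseLocation if tagged "Noise".
; The sight branch checks neither actor type nor whether sensing succeeded, so losing sight also writes the actor rather than clearing the key.
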(event `self.AIPerceptionComponent.OnTargetPerceptionUpdated`
  (params (Actor :type "Actor Object Reference") (Stimulus :type "AIStimulus Structure"))
  (bind (_age _expirationage _strength _stimuluslocation _receiverlocation _tag) (break `AIStimulus` Stimulus))
  (bind _returnvalue (`AIPerceptionSystem.GetSenseClassForStimulus` Stimulus))
  (if (== _returnvalue "/Script/AIModule.AISense_Sight")
    (`BlackboardComponent.SetValueAsObject` (`self.Blackboard`) "PlayerActor" Actor)
    (elif (== _returnvalue "/Script/AIModule.AISense_Hearing")
      (if (== _tag "Noise")
        (`BlackboardComponent.SetValueAsVector` (`self.Blackboard`) "NoiseLocation" _stimuluslocation)))))

(fn `UserConstructionScript`)