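; Behavior tree task for deer AI that picks a point to flee to from a heard noise.
; It scales the normalized direction from blackboard NoiseLocation to the pawn and uses it directly as a navmesh search origin, without adding the pawn's location.
; A random navigable point near that origin is written to LocationToRunTo.
; The task's success comes from a separate evaluation of the same random query.
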(event `self.ReceiveExecuteAI`
  (params (OwnerController :type "AIController Object Reference") (ControlledPawn :type "Pawn Object Reference"))
  (bind _returnvalue (`AIBlueprintHelperLibrary.GetBlackboard` ControlledPawn))
  (bind (_randomlocation _returnvalue_2) (`NavigationSystemV1.K2_GetRandomLocationInNavigableRadius` (* (`KismetMathLibrary.Normal` (- (`Actor.K2_GetActorLocation` ControlledPawn) (`BlackboardComponent.GetValueAsVector` _returnvalue "NoiseLocation"))) 1000.0) 100.0 null null))
  (`BlackboardComponent.SetValueAsVector` _returnvalue "LocationToRunTo" _randomlocation)
  (`self.FinishExecute` _returnvalue_2))