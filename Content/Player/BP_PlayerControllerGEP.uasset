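; BP_PlayerControllerGEP is a player controller Blueprint that owns and opens the options menu UI.
; On BeginPlay, after a short delay, it creates the options menu widget for player 0, stores it, adds it to the viewport and initializes it with that controller.
; The OnOptionsMenuPressed event opens the stored widget if it is valid.
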(event `self.ReceiveBeginPlay`
  ;[1 1 1] Initialize Options Menu UI
  (`KismetSystemLibrary.Delay` 0.2)
  (bind _returnvalue (`|CreateWidget` "/Game/UI/OptionsMenuUIWidget.OptionsMenuUIWidget_C" (`GameplayStatics.GetPlayerController` 0)))
  (bind _output_get (set `self.OptionsMenuWidget` _returnvalue))
  (`UserWidget.AddToViewport` _output_get 0)
  (`/Game/UI/OptionsMenuUIWidget.InitializeOptionsMenu_Event` (`self.OptionsMenuWidget`) (`GameplayStatics.GetPlayerController` 0)))

(event `self.OnOptionsMenuPressed`
  (bind _optionsmenuwidget (`self.OptionsMenuWidget`))
  ;[1 1 1] Open Options Menu
  (`/Engine/EditorBlueprintResources/StandardMacros.IsValid` _optionsmenuwidget
    (:`Is Valid`
      (`/Game/UI/OptionsMenuUIWidget.OpenMenu` _optionsmenuwidget))))

(fn `UserConstructionScript`)