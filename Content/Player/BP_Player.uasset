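; BP_Player is the player Blueprint, which sets up the inventory UI and opens it from input.
; On BeginPlay, after a very brief delay, it creates the inventory widget, adds it to the viewport and initializes it with its inventory component and player controller.
; The Inventory input action calls the widget's toggle event, always passing true, once the widget is valid.
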(event `InputAction|Inventory`
  (params (Key :type "Key Structure"))
  (bind _inventorywidget (`self.InventoryWidget`))
  ;[1 1 1] Open Inventory UI
  (:`Pressed`
    (if (`KismetSystemLibrary.IsValid` _inventorywidget)
      (`/Game/UI/Inventory/Widget_Inventory.ToggleInventory_Event` _inventorywidget true))))

(event `self.ReceiveBeginPlay`
  ;[1 1 1] Add Inventory Widget To Scene
  (`KismetSystemLibrary.Delay` 0.001)
  (bind _returnvalue (`self.GetPlayerControllerGEP`))
  (bind _returnvalue_2 (`|CreateWidget` "/Game/UI/Inventory/Widget_Inventory.Widget_Inventory_C" _returnvalue))
  (bind _output_get (set `self.InventoryWidget` _returnvalue_2))
  (`UserWidget.AddToViewport` _output_get 0)
  (`/Game/UI/Inventory/Widget_Inventory.InitializeInvUI_Event` (`self.InventoryWidget`) (`self.InventoryComponent`) (`GameplayStatics.GetPlayerController` 0)))

(fn `UserConstructionScript`)